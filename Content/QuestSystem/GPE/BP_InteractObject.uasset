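; Base interactable quest actor that runs an overridable ExecuteInteraction, optionally requiring an item from the player's inventory.
; A sphere overlap toggles the WBP_PressE prompt, set up at BeginPlay with the required item's icon.
; A DoOnce gates item-based interactions; consuming the item either re-arms it or permanently hides the prompt.
; GetIfValidateInteract derives completion from that hidden-prompt flag.
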(event `self.ReceiveBeginPlay`
  (bind _aswbp_press_e (cast `/Game/UI/WBP_PressE` (`WidgetComponent.GetWidget` (`self.Widget`)) :!pure true))
  ;[0.006151 0 0.5208] Adapt Ui element for interact button whith item needed for interaction
  (`Image.SetBrush` (`/Game/UI/WBP_PressE.Item` _aswbp_press_e) (make `SlateBrush` "Image" "NoTile" "NoMirror" (make `DeprecateSlateVector2D` 100.0 100.0) (struct) (struct :`SpecifiedColor` (struct :`R` 1.0 :`G` 1.0 :`B` 1.0 :`A` 1.0) :`ColorUseRule` "UseColor_Specified") (struct :`CornerRadii` (struct) :`Color` (struct :`SpecifiedColor` (struct) :`ColorUseRule` "UseColor_Specified") :`RoundingType` "HalfHeightRadius") (defaults `Object` (`self.ItemNeed`))))
  (set `/Game/UI/WBP_PressE.needItem?` (`self.NeedItem?`) _aswbp_press_e))

(event `/Game/QuestSystem/Interface/BPI_Interact.Interact`
  (params (Inv :type "Array of /Game/QuestSystem/Reward/BP_Item Class Reference (by ref)"))
  (bind _returnvalue (`KismetArrayLibrary.Array_Find` Inv (`self.ItemNeed`)))
  ;[1 0.4107 0] Inteact system
  (if (`self.NeedItem?`)
    ;;[0 0.5812 1] Execute interaction if player has the good item in his inventory
    (if (!= _returnvalue -1)
      (`/Engine/EditorBlueprintResources/StandardMacros.DoOnce` false :!label _label
        (:`Completed`
          (`self.ExecuteInteraction`)
          (if (`self.ConsumeItem?`)
            (`/Game/FirstPerson/Blueprints/BP_FirstPersonCharacter.RemoveItem` (cast `/Game/FirstPerson/Blueprints/BP_FirstPersonCharacter` (`GameplayStatics.GetPlayerCharacter` 0) :!pure true) _returnvalue)
            (if (`self.CanInteractAgain?`)
              (`self.InteractAgain`)
              (else
                (`SceneComponent.SetVisibility` (`self.Widget`) false false)
                (set `self.ShowPressE?` false)))))))
    (else
      (`self.ExecuteInteraction`))))

(event `InteractAgain`
  ;[1 0.4107 0] Inteact system
  ;;[0 0.5812 1] Execute interaction if player has the good item in his inventory
  (goto _label :!via `Reset`))

(event `ExecuteInteraction`
  ;[1 0.4107 0] Inteact system
)

(event `self.Sphere.OnComponentBeginOverlap`
  (params (OverlappedComponent :type "PrimitiveComponent Object Reference") (OtherActor :type "Actor Object Reference") (OtherComp :type "PrimitiveComponent Object Reference") (OtherBodyIndex :type Integer) (bFromSweep :type Boolean) (SweepResult :type "HitResult Structure (by ref)"))
  ;[0 0 0] Show/hide interact button when playre enter/exit sphere detection zone
  (if (and (== OtherActor (`GameplayStatics.GetPlayerPawn` 0)) (`self.ShowPressE?`))
    (`SceneComponent.SetVisibility` (`self.Widget`) true false)))

(event `self.Sphere.OnComponentEndOverlap`
  (params (OverlappedComponent :type "PrimitiveComponent Object Reference") (OtherActor :type "Actor Object Reference") (OtherComp :type "PrimitiveComponent Object Reference") (OtherBodyIndex :type Integer))
  ;[0 0 0] Show/hide interact button when playre enter/exit sphere detection zone
  (if (and (== OtherActor (`GameplayStatics.GetPlayerPawn` 0)) (`self.ShowPressE?`))
    (`SceneComponent.SetVisibility` (`self.Widget`) false false)))

(fn `GetIfValidateInteract`
  (returns (`ShowPressE?` :type Boolean))
  (return (not (`self.ShowPressE?`))))

(fn `UserConstructionScript`)