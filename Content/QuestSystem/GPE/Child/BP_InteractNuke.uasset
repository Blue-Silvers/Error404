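; BP_InteractNuke is a child interactable in the quest system whose interaction ends the game with a victory screen.
; ExecuteInteraction creates WBP_Victory, adds it to the viewport and pauses the game.
; It then shows the mouse cursor and switches the first player controller to UI-only input, focused on the widget's New Game button.
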(event `self.ExecuteInteraction`
  (bind _returnvalue (`GameplayStatics.GetPlayerController` 0))
  ;[1 1 1] Win screen
  (bind _returnvalue_2 (`|CreateWidget` "/Game/UI/Menus/Viewport/WBP_Victory.WBP_Victory_C" (`GameplayStatics.GetPlayerController` 0)))
  (`UserWidget.AddToViewport` _returnvalue_2 0)
  (`GameplayStatics.SetGamePaused` true)
  (set `PlayerController.bShowMouseCursor` true _returnvalue)
  (`WidgetBlueprintLibrary.SetInputMode_UIOnlyEx` _returnvalue (`/Game/UI/Menus/Viewport/WBP_Victory.NewGameButton` _returnvalue_2)))

(fn `UserConstructionScript`
  (`parent.UserConstructionScript`))