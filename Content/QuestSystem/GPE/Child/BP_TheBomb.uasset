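; BP_TheBomb is a quest interactable that wins the game once all three bomb pieces are repaired.
; On ExecuteInteraction it waits one tick, then reads the validated-interaction state of three child-actor BP_InteractObject parts.
; If all three are validated, it shows the WBP_Victory widget, pauses the game, and switches to UI-only input with the cursor visible and the New Game button focused.
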(event `self.ExecuteInteraction`
  (bind _returnvalue (`GameplayStatics.GetPlayerController` 0))
  ;[0 0 0] Check if all bomb pieces are repear
  (`KismetSystemLibrary.DelayUntilNextTick`)
  (bind _showpresse_ (`self.GetIfValidateInteract` (cast `/Game/QuestSystem/GPE/BP_InteractObject` (`ChildActorComponent.ChildActor` (`self.Part1`)) :!pure true)))
  (bind _showpresse__2 (`self.GetIfValidateInteract` (cast `/Game/QuestSystem/GPE/BP_InteractObject` (`ChildActorComponent.ChildActor` (`self.Part2`)) :!pure true)))
  (bind _showpresse__3 (`self.GetIfValidateInteract` (cast `/Game/QuestSystem/GPE/BP_InteractObject` (`ChildActorComponent.ChildActor` (`self.Part3`)) :!pure true)))
  (if (and _showpresse__3 _showpresse__2 _showpresse_)
    ;[1 1 1] Win screen
    (bind _returnvalue_2 (`|CreateWidget` "/Game/UI/Menus/Viewport/WBP_Victory.WBP_Victory_C" (`GameplayStatics.GetPlayerController` 0)))
    (`UserWidget.AddToViewport` _returnvalue_2 0)
    (`GameplayStatics.SetGamePaused` true)
    (set `PlayerController.bShowMouseCursor` true _returnvalue)
    (`WidgetBlueprintLibrary.SetInputMode_UIOnlyEx` _returnvalue (`/Game/UI/Menus/Viewport/WBP_Victory.NewGameButton` _returnvalue_2))))

(fn `UserConstructionScript`)