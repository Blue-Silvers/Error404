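; BP_PickUp is a dropped item pickup that the player collects by touching it.
; On BeginPlay it spawns ChildClass as a child actor, copies that BP_Item's mesh and scale, launches the mesh along Foward, and becomes pickable one second later.
; Player overlap with the mesh or sphere calls AddInInventoryMessage on the player character with ChildClass, destroying the pickup when that call returns false.
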(event `self.ReceiveBeginPlay`
  (bind _childactor (`self.ChildActor`))
  (`ChildActorComponent.SetChildActorClass` _childactor (`self.ChildClass`))
  (bind _asbp_item (cast `/Game/QuestSystem/Reward/BP_Item` (`ChildActorComponent.ChildActor` _childactor)))
  (bind _itemmesh (`/Game/QuestSystem/Reward/BP_Item.ItemMesh` _asbp_item))
  (`StaticMeshComponent.SetStaticMesh` (`self.Mesh`) (`StaticMeshComponent.StaticMesh` _itemmesh))
  (`SceneComponent.SetWorldScale3D` (`self.Mesh`) (`SceneComponent.RelativeScale3D` _itemmesh))
  (`PrimitiveComponent.AddImpulse` (`self.Mesh`) (* (`self.Foward`) 2000.0) "None" false)
  (`KismetSystemLibrary.Delay` 1.0)
  (set `self.IsPickable` true))

(event `self.Mesh.OnComponentBeginOverlap`
  (params (OverlappedComponent :type "PrimitiveComponent Object Reference") (OtherActor :type "Actor Object Reference") (OtherComp :type "PrimitiveComponent Object Reference") (OtherBodyIndex :type Integer) (bFromSweep :type Boolean) (SweepResult :type "HitResult Structure (by ref)"))
  (bind _returnvalue (`GameplayStatics.GetPlayerCharacter` 0))
  (if (and (== OtherActor _returnvalue) (`self.IsPickable`))
    (bind _inventoryfull (message `/Game/QuestSystem/Interface/BPI_player.AddInInventory` _returnvalue (`self.ChildClass`) :!label _label))
    (if (not _inventoryfull)
      (`self.K2_DestroyActor`))))

(event `self.Sphere.OnComponentBeginOverlap`
  (params (OverlappedComponent :type "PrimitiveComponent Object Reference") (OtherActor :type "Actor Object Reference") (OtherComp :type "PrimitiveComponent Object Reference") (OtherBodyIndex :type Integer) (bFromSweep :type Boolean) (SweepResult :type "HitResult Structure (by ref)"))
  (if (and (`self.IsPickable`) (== OtherActor (`GameplayStatics.GetPlayerCharacter` 0)))
    (goto _label)))

(fn `UserConstructionScript`)