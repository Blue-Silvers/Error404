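; BP_WeaponLaserGun is a laser weapon that charges a beam, then damages everything along the player camera's forward direction.
; UseTrigger passes a DoOnce, spawns a Niagara beam, makes player noise and runs a timeline that widens it.
; When charged, a debug-drawn multi-object line trace damages every hit, then the beam is destroyed and ResetWeapon re-arms after a fire-rate delay.
; The timeline's vector parameter update has its name set to None.
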(event `/Game/QuestSystem/Interface/BPI_Items.UseTrigger`
  (bind _returnvalue (`GameplayStatics.GetPlayerCharacter` 0))
  (bind _laser (`self.Laser`))
  (bind _returnvalue_2 (`SceneComponent.K2_GetComponentLocation` (`self.Laser`)))
  (`/Engine/EditorBlueprintResources/StandardMacros.DoOnce` false :!label _label
    (:`Completed`
      (bind _returnvalue_3 (`AddComponent|NODE_AddNiagaraComponent-1` :`RelativeTransform` (`self.LaserOffset`)))
      (set `self.Laser` _returnvalue_3)
      (`Pawn.PawnMakeNoise` _returnvalue 1.0 (0.0 0.0 0.0) true _returnvalue)
      (bind (_direction _newtrack_0 _newtrack_1) (`Timeline|LaserCharge` :!via `PlayFromStart`)
        (:`Update`
          (`FXSystemComponent.SetFloatParameter` _laser "Beam Width" (`KismetMathLibrary.Lerp` 0.1 10.0 _newtrack_0))
          (`FXSystemComponent.SetVectorParameter` _laser "None" (`KismetMathLibrary.VLerp` (1000.0 0.0 0.0) (10000.0 0.0 0.0) _newtrack_1)))
        (:`Finished`
          (bind _outhits (`KismetSystemLibrary.LineTraceMultiForObjects` :`Start` _returnvalue_2 :`End` (+ _returnvalue_2 (* (`SceneComponent.GetForwardVector` (`PlayerCameraManager.TransformComponent` (`GameplayStatics.GetPlayerCameraManager` 0))) 10000.0)) :`ObjectTypes` (`self.Targets`) :`DrawDebugType` "ForDuration"))
          (for _array_element _outhits
            (`GameplayStatics.ApplyDamage` (`.HitActor` (`GameplayStatics.BreakHitResult` _array_element)) (`self.Damage`)))
          (`KismetSystemLibrary.Delay` 0.1)
          (`ActorComponent.K2_DestroyComponent` (`self.Laser`))
          (`self.ResetWeapon`))))))

(event `ResetWeapon`
  (`KismetSystemLibrary.Delay` (/ 1.0 (`self.FireRate`)))
  (goto _label :!via `Reset`))

(fn `UserConstructionScript`
  (`parent.UserConstructionScript`))