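; Shotgun weapon Blueprint that fires a burst of pellets when UseTrigger is called.
; Each shot spawns fifteen BP_ShotgunProjectile actors from the offset item mesh location, randomly spreading them around the camera rotation and passing Damage to each.
; It also emits pawn noise, plays a firing sound and plays a montage on the first-person mesh.
; A DoOnce gate, reset after a delay derived from FireRate, limits the firing rate.
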(event `/Game/QuestSystem/Interface/BPI_Items.UseTrigger`
  (bind _returnvalue (`GameplayStatics.GetPlayerCharacter` 0))
  (bind (_returnvalue_roll _returnvalue_pitch _returnvalue_yaw) (`KismetMathLibrary.BreakRotator` (`PlayerCameraManager.GetCameraRotation` (`GameplayStatics.GetPlayerCameraManager` 0))))
  (bind _returnvalue_2 (`KismetMathLibrary.MakeRotator` _returnvalue_roll (+ _returnvalue_pitch (`KismetMathLibrary.RandomFloatInRange` -7.5 7.5)) (+ _returnvalue_yaw (`KismetMathLibrary.RandomFloatInRange` -7.5 7.5))))
  (bind _returnvalue_3 (+ (`SceneComponent.K2_GetComponentLocation` (`self.ItemMesh`)) (`KismetMathLibrary.GreaterGreater_VectorRotator` (`self.ProjectileOffset`) _returnvalue_2)))
  (`/Engine/EditorBlueprintResources/StandardMacros.DoOnce` false :!label _label
    (:`Completed`
      (`Pawn.PawnMakeNoise` _returnvalue 1.0 (0.0 0.0 0.0) true _returnvalue)
      (for _ (range 15)
        (`|SpawnActorFromClass` "/Game/QuestSystem/Reward/WIPWeapons/BP_ShotgunProjectile.BP_ShotgunProjectile_C" (`KismetMathLibrary.MakeTransform` _returnvalue_3 _returnvalue_2 (0.3 0.3 0.3)) "Undefined" "OverrideRootScale" null (`self.Damage`) null))
      (`GameplayStatics.PlaySoundAtLocation` "/Game/FPWeapon/Audio/FirstPersonTemplateWeaponFire02.FirstPersonTemplateWeaponFire02" _returnvalue_3 (struct) 1.0 1.0 0.0 null null null null) ; Play firing sound
      (bind _asbp_first_person_character (cast `/Game/FirstPerson/Blueprints/BP_FirstPersonCharacter` _returnvalue))
      (`AnimInstance.Montage_Play` (`SkeletalMeshComponent.GetAnimInstance` (`/Game/FirstPerson/Blueprints/BP_FirstPersonCharacter.FirstPersonMesh` _asbp_first_person_character)) "/Game/FirstPersonArms/Animations/FP_Rifle_Shoot_Montage.FP_Rifle_Shoot_Montage" 1.0 "MontageLength" 0.0 true)
      (`self.ResetShoot`))))

(event `ResetShoot`
  (`KismetSystemLibrary.Delay` (/ 1.0 (`self.FireRate`)))
  (goto _label :!via `Reset`))

(fn `UserConstructionScript`
  (`parent.UserConstructionScript`))