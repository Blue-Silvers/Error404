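; Base turret enemy that detects the player with PawnSensing, turns to face them and fires through an empty Shoot event.
; Sensing interval derives from FireRate; sightings outside LockAngle play an easing timeline scaled by RotationSpeed before firing, otherwise it fires directly.
; The timeline rotates the Scene component and actor yaw, and a short delay gates shots.
; Tick keeps a Niagara laser visible, line-tracing to set beam length.
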(event `self.ReceiveBeginPlay`
  (`parent.ReceiveBeginPlay`)
  (`TimelineComponent.SetPlayRate` (`self.Ease_Rotation`) (`self.RotationSpeed`))
  (`PawnSensingComponent.SetSensingInterval` (`self.PawnSensing`) (/ 1.0 (`self.FireRate`)))
  (`SkeletalMeshComponent.PlayAnimation` (`self.SK_SciFi_ToiletMech_Skin1`) "/Game/SciFi_ToiletMech/Animation/Anim_SciFi_ToiletMech_Idle1_Toilet.Anim_SciFi_ToiletMech_Idle1_Toilet" true)
  (`|ExecutionSequence`
    (:`then_0`
      (`SceneComponent.SetVisibility` (`self.Niagara`) false false))))

(event `self.PawnSensing.OnSeePawn`
  (params (Pawn :type "Pawn Object Reference"))
  (bind (_returnvalue_roll _returnvalue_pitch _returnvalue_yaw) (`KismetMathLibrary.BreakRotator` (`self.K2_GetActorRotation`)))
  (bind _scene (`self.Scene`))
  (bind (_returnvalue_roll_2 _returnvalue_pitch_2 _returnvalue_yaw_2) (`KismetMathLibrary.BreakRotator` (`KismetMathLibrary.FindLookAtRotation` (`self.K2_GetActorLocation`) (`self.K2_GetActorLocation` Pawn))))
  (bind _returnvalue (/ (`self.LockAngle`) 2.0))
  ;[0 0 0] Player Detection and Shoot
  ;;[1 1 1] Check if Detected pawn is the player and if it already well rotated
  (if (== (`GameplayStatics.GetPlayerPawn` 0) Pawn)
    (if (not (and (>= _returnvalue_yaw (- _returnvalue_yaw_2 _returnvalue)) (<= _returnvalue_yaw (+ _returnvalue_yaw_2 _returnvalue))))
      ;;[1 1 1] Rotates the turret toward the player
      (bind (_direction _newtrack_0) (`Timeline|Ease_Rotation` :!via `PlayFromStart`)
        (:`Update`
          (bind _returnvalue_2 (`KismetMathLibrary.RLerp` (`SceneComponent.K2_GetComponentRotation` _scene) (`KismetMathLibrary.FindLookAtRotation` (`SceneComponent.K2_GetComponentLocation` _scene) (`self.K2_GetActorLocation` Pawn)) _newtrack_0 true))
          (`SceneComponent.K2_SetWorldRotation` _scene _returnvalue_2 false false)
          (`self.K2_SetActorRotation` (`KismetMathLibrary.MakeRotator` 0.0 0.0 (.yaw _returnvalue_2))))
        (:`Finished`
          ;;[1 1 1] Shoot the player
          (if (`self.canShoot?`) :!label _label
            (set `self.canShoot?` false)
            (`self.Shoot`)
            (`KismetSystemLibrary.Delay` 0.1)
            (set `self.canShoot?` true))))
      (else
        (goto _label)))))

(event `Shoot`)

(event `LaserPointer`
  (`SceneComponent.SetVisibility` (`self.Niagara`) true false)
  (set `self.LineTraceActivated?` true))

(event `self.ReceiveTick`
  (params (DeltaSeconds :type "Float (single-precision)"))
  (`parent.ReceiveTick` DeltaSeconds)
  (`self.LaserPointer`)
  (if (`self.LineTraceActivated?`)
    (`self.LineTrace`)))

(event `LineTrace`
  (bind _niagara (`self.Niagara`))
  (bind _returnvalue (`SceneComponent.K2_GetComponentLocation` _niagara))
  (bind (_outhit _returnvalue_2) (`KismetSystemLibrary.LineTraceSingle` :`Start` _returnvalue :`End` (+ _returnvalue (* (`SceneComponent.GetForwardVector` _niagara) (`self.EndOfLine`))) :`TraceChannel` "TraceTypeQuery1" :`DrawTime` 0.1))
  (if _returnvalue_2
    (`FXSystemComponent.SetVectorParameter` (`self.Niagara`) "Beam End" (`KismetMathLibrary.MakeVector` (`.Distance` (`GameplayStatics.BreakHitResult` _outhit))))
    (else
      (`FXSystemComponent.SetVectorParameter` (`self.Niagara`) "Beam End" (`KismetMathLibrary.MakeVector` (`self.EndOfLine`))))))

(fn `UserConstructionScript`
  (`parent.UserConstructionScript`))