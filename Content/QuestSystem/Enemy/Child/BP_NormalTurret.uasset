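; BP_NormalTurret is a child turret enemy in the quest system that fires electric balls.
; On the Shoot event it spawns a BP_ElectricBall at its Scene component's world transform and passes its Damage value to the projectile's BulletDamage.
; Its construction script only calls the parent, and its other events are disabled stubs.
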(event `self.Shoot`
  (bind _returnvalue (`|SpawnActorFromClass` "/Game/QuestSystem/Enemy/Bullets/BP_ElectricBall.BP_ElectricBall_C" (`SceneComponent.K2_GetComponentToWorld` (`self.Scene`)) "Undefined" "MultiplyWithRoot" null null))
  (set `/Game/QuestSystem/Enemy/Bullets/BP_ElectricBall.BulletDamage` (`self.Damage`) _returnvalue))

(fn `UserConstructionScript`
  (`parent.UserConstructionScript`))