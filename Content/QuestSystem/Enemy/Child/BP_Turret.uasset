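; BP_Turret is a child enemy Blueprint for a stationary turret that detects the player, turns toward them and shoots electric balls.
; PawnSensing runs at an interval derived from FireRate, so each sighting of the player drives a shot.
; If yaw is outside a 10-degree tolerance, a timeline scaled by RotationSpeed eases the rotation before firing; otherwise it fires immediately.
; Each shot spawns a BP_ElectricBall at the turret's transform and passes it the turret's Damage.
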(event `self.ReceiveBeginPlay`
  (`parent.ReceiveBeginPlay`)
  (`TimelineComponent.SetPlayRate` (`self.Ease_Rotation`) (`self.RotationSpeed`))
  (`PawnSensingComponent.SetSensingInterval` (`self.PawnSensing`) (/ 1.0 (`self.FireRate`))))

(event `self.PawnSensing.OnSeePawn`
  (params (Pawn :type "Pawn Object Reference"))
  (bind (_returnvalue_roll _returnvalue_pitch _returnvalue_yaw) (`KismetMathLibrary.BreakRotator` (`self.K2_GetActorRotation`)))
  (bind (_returnvalue_roll_2 _returnvalue_pitch_2 _returnvalue_yaw_2) (`KismetMathLibrary.BreakRotator` (`KismetMathLibrary.FindLookAtRotation` (`self.K2_GetActorLocation`) (`self.K2_GetActorLocation` Pawn))))
  ;[0 0 0] Player Detection and Shoot
  ;;[1 1 1] Check if Detected pawn is the player and if it already well rotated
  (if (== (`GameplayStatics.GetPlayerPawn` 0) Pawn)
    (if (not (and (>= _returnvalue_yaw (- _returnvalue_yaw_2 10.0)) (<= _returnvalue_yaw (+ _returnvalue_yaw_2 10.0))))
      ;;[1 1 1] Rotates the turret toward the player
      (bind (_direction _newtrack_0) (`Timeline|Ease_Rotation` :!via `PlayFromStart`)
        (:`Update`
          (`self.K2_SetActorRotation` (`KismetMathLibrary.RLerp` (`self.K2_GetActorRotation`) (`KismetMathLibrary.FindLookAtRotation` (`self.K2_GetActorLocation`) (`self.K2_GetActorLocation` Pawn)) _newtrack_0 true)))
        (:`Finished`
          ;;[1 1 1] Shoot the player
          (bind _returnvalue (`|SpawnActorFromClass` "/Game/QuestSystem/Enemy/Bullets/BP_ElectricBall.BP_ElectricBall_C" (`self.GetTransform`) "Undefined" "MultiplyWithRoot" null null :!label _label))
          (set `/Game/QuestSystem/Enemy/Bullets/BP_ElectricBall.BulletDamage` (`self.Damage`) _returnvalue)))
      (else
        (goto _label)))))

(fn `UserConstructionScript`
  (`parent.UserConstructionScript`))