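; BP_MeleeEnemy is a child enemy Blueprint that performs a melee attack against the first-person character.
; It plays a looping run animation from BeginPlay, setting animations directly on the mesh.
; The Attack event plays an attack animation, waits briefly, then sphere-traces at a scene component's location and applies damage if it hits the player.
; Debug strings report the damage or hit actor, and the run animation resumes after another delay.
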(event `self.ReceiveBeginPlay`
  (`parent.ReceiveBeginPlay`)
  (`SkeletalMeshComponent.PlayAnimation` (`self.Mesh`) "/Game/SciFi_ToiletMech/Animation/Anim_SciFi_ToiletMech_Run.Anim_SciFi_ToiletMech_Run" true))

(event `Attack`
  (bind _damage (`self.Damage`))
  (bind _mesh (`self.Mesh`))
  (bind _returnvalue (`SceneComponent.K2_GetComponentLocation` (`self.Scene`)))
  (`SkeletalMeshComponent.PlayAnimation` _mesh "/Game/SciFi_ToiletMech/Animation/Anim_SciFi_ToiletMech_Attack3.Anim_SciFi_ToiletMech_Attack3" false)
  (`KismetSystemLibrary.Delay` 1.0)
  (`|ExecutionSequence`
    (:`then_0`
      (bind _outhit (`KismetSystemLibrary.SphereTraceSingleForObjects` _returnvalue _returnvalue 200.0 (`self.Object Types`)))
      (bind (_bblockinghit _binitialoverlap _time _distance _location _impactpoint _normal _impactnormal _physmat _hitactor) (`GameplayStatics.BreakHitResult` _outhit))
      (bind _asbp_first_person_character (cast `/Game/FirstPerson/Blueprints/BP_FirstPersonCharacter` _hitactor)
        (:`then`
          (`GameplayStatics.ApplyDamage` _asbp_first_person_character _damage)
          (`KismetSystemLibrary.PrintString` (`KismetStringLibrary.Conv_DoubleToString` _damage)))
        (:`CastFailed`
          (`KismetSystemLibrary.PrintString` (`KismetSystemLibrary.GetDisplayName` _hitactor)))))
    (:`then_1`
      (`KismetSystemLibrary.Delay` 1.0)
      (`SkeletalMeshComponent.PlayAnimation` _mesh "/Game/SciFi_ToiletMech/Animation/Anim_SciFi_ToiletMech_Run.Anim_SciFi_ToiletMech_Run" true))))

(fn `UserConstructionScript`
  (`parent.UserConstructionScript`))