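; BP_TriTurret is a child enemy turret that fires a three-projectile spread of electric balls.
; Its Shoot event spawns three BP_ElectricBall actors at the Scene component's transform, one straight ahead and two yawed half of ShotWideness to either side.
; Each projectile receives the turret's Damage as its BulletDamage.
; BeginPlay, overlap and Tick are unused stubs, and the construction script just calls the parent.
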(event `self.Shoot`
  (bind _returnvalue (`SceneComponent.K2_GetComponentToWorld` (`self.Scene`)))
  (bind _returnvalue_2 (/ (`self.ShotWideness`) 2.0))
  (bind _location (.location _returnvalue))
  (bind _scale (.scale _returnvalue))
  (bind _roll (.roll (.rotation _returnvalue)))
  (bind _pitch (.pitch (.rotation _returnvalue)))
  (bind _yaw (.yaw (.rotation _returnvalue)))
  (bind _returnvalue_3 (`|SpawnActorFromClass` "/Game/QuestSystem/Enemy/Bullets/BP_ElectricBall.BP_ElectricBall_C" _returnvalue "Undefined" "MultiplyWithRoot" null null))
  (set `/Game/QuestSystem/Enemy/Bullets/BP_ElectricBall.BulletDamage` (`self.Damage`) _returnvalue_3)
  (bind _returnvalue_4 (`|SpawnActorFromClass` "/Game/QuestSystem/Enemy/Bullets/BP_ElectricBall.BP_ElectricBall_C" (`KismetMathLibrary.MakeTransform` _location (`KismetMathLibrary.MakeRotator` _roll _pitch (+ _yaw _returnvalue_2)) _scale) "Undefined" "MultiplyWithRoot" null null))
  (set `/Game/QuestSystem/Enemy/Bullets/BP_ElectricBall.BulletDamage` (`self.Damage`) _returnvalue_4)
  (bind _returnvalue_5 (`|SpawnActorFromClass` "/Game/QuestSystem/Enemy/Bullets/BP_ElectricBall.BP_ElectricBall_C" (`KismetMathLibrary.MakeTransform` _location (`KismetMathLibrary.MakeRotator` _roll _pitch (- _yaw _returnvalue_2)) _scale) "Undefined" "MultiplyWithRoot" null null))
  (set `/Game/QuestSystem/Enemy/Bullets/BP_ElectricBall.BulletDamage` (`self.Damage`) _returnvalue_5))

(fn `UserConstructionScript`
  (`parent.UserConstructionScript`))