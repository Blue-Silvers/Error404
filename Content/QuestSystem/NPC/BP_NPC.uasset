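; BP_NPC is a quest-giving NPC that shows its quest dialogue when talked to and then hands the quest to the player.
; The HaveMission marker is visible at start only when a quest DataAsset is assigned.
; Each Talk call, while the quest is incomplete, advances one line in a WBP_Dialogue widget.
; Past the last line it closes the widget, resets, and a DoOnce adds the quest to BP_FirstPersonCharacter and hides the marker.
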(event `self.ReceiveBeginPlay`
  (bind _havemission (`self.HaveMission`))
  (`/Engine/EditorBlueprintResources/StandardMacros.IsValid` (`self.DataAsset`)
    (:`Is Valid`
      (`SceneComponent.SetVisibility` _havemission true true))
    (:`Is Not Valid`
      (`SceneComponent.SetVisibility` _havemission false true))))

(event `GiveQuest`
  (`/Game/FirstPerson/Blueprints/BP_FirstPersonCharacter.AddQuest` (cast `/Game/FirstPerson/Blueprints/BP_FirstPersonCharacter` (`GameplayStatics.GetPlayerCharacter` 0) :!pure true) (`self.DataAsset`))
  (`SceneComponent.SetVisibility` (`self.HaveMission`) false true))

(event `/Game/QuestSystem/NPC/BPI_Dialogue.Talk`
  (bind _index (`self.Index`))
  (bind (_queststruct_title _queststruct_dialogue) (break `/Game/QuestSystem/DataAssest/Blueprint/Data/Struct_Quest` (`/Game/QuestSystem/DataAssest/Blueprint/BP_QuestDataAssest.QuestStruct` (`self.DataAsset`))))
  (`/Engine/EditorBlueprintResources/StandardMacros.IsValid` (`self.DataAsset`)
    (:`Is Valid`
      (if (not (`self.QuestComplete`))
        (`/Engine/EditorBlueprintResources/StandardMacros.IsValid` (`self.UI`)
          (:`Is Valid`
            (`Widget.RemoveFromParent` (stale _output_get)))
          (:`Is Not Valid`
            (bind _returnvalue (`|CreateWidget` "/Game/UI/Dialogue/WBP_Dialogue.WBP_Dialogue_C"))
            (bind _output_get (set `self.UI` _returnvalue))))
        (`UserWidget.AddToViewport` _output_get 0)
        (`/Game/UI/Dialogue/WBP_Dialogue.SetNewDialogue` _output_get (`KismetTextLibrary.Conv_StringToText` (`|GetArrayItem` _queststruct_dialogue _index)))
        (if (>= _index (`KismetArrayLibrary.Array_Length` _queststruct_dialogue))
          (set `self.Index` 0)
          (`Widget.RemoveFromParent` (`self.UI`))
          (`/Engine/EditorBlueprintResources/StandardMacros.DoOnce` false
            (:`Completed`
              (`self.GiveQuest`)))
          (else
            (`/Engine/EditorBlueprintResources/StandardMacros.IncrementInt` _index)))))))

(fn `UserConstructionScript`)